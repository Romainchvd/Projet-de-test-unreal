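; BP_Collectible is a spinning pickup that awards one point to the player when collected.
; It rotates a fixed step every Tick and caches GM_SuperGameMode on BeginPlay.
; When the player pawn overlaps its sphere, it adds score on BP_SuperPlayerState, calls PointsStatues on the game mode's Interface, then destroys itself.
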(event OnComponentBeginOverlap(Sphere)
  (params (OverlappedComponent :type Primitive%20Component%20Object%20Reference) (OtherActor :type Actor%20Object%20Reference) (OtherComp :type Primitive%20Component%20Object%20Reference) (OtherBodyIndex :type Integer) (bFromSweep :type Boolean) (SweepResult :type Hit%20Result%20Structure%20%28by%20ref%29))
  (if (== OtherActor (Game|Player|GetPlayerPawn 0))
    (Utilities|FlowControl|Sequence
      (:then_0
        (bind _asbp_super_player_state (Utilities|Casting|CastToBP_SuperPlayerState (Game|GetPlayerState 0)))
        (Default|AddScore _asbp_super_player_state 1)
        (Default|PointsStatues (Variables|/Game/Blueprint/GM_SuperGameMode.GM_SuperGameMode_C|Getinterface (stale EventBeginPlay _asgm_super_game_mode))))
      (:then_1
        (Actor|DestroyActor)))))

(event EventBeginPlay
  (bind _asgm_super_game_mode (Utilities|Casting|CastToGM_SuperGameMode (Game|GetGameMode))))

(event Collision|EventActorBeginOverlap
  (params (OtherActor :type Actor%20Object%20Reference)))

(event EventTick
  (params (DeltaSeconds :type Float%20%28single-precision%29))
  (Transformation|AddActorLocalRotation "0.000000,1.000000,0.000000" false false))

(fn ConstructionScript)