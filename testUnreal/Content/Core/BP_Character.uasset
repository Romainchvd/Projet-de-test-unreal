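; BP_Character is a character Blueprint that holds basic health and death state.
; UpdateHealthPoints adds a signed delta to HealthPoints and always returns zero, without triggering the death check.
; UpdateIsDead sets IsDead from whether health is at or below zero, but calls itself before setting it true, so that branch recurses endlessly.
; BeginPlay, Tick and overlap events are empty, and nothing connected in this graph starts either update.
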(event Custom|UpdateIsDead
  (if (<= (Variables|Default|GetHealthPoints) 0.0)
    (CallFunction|UpdateIsDead)
    (Variables|Default|SetisDead true)
    (else
      (Variables|Default|SetisDead false))))

(event EventBeginPlay)

(event Collision|EventActorBeginOverlap
  (params (OtherActor :type Actor%20Object%20Reference)))

(event EventTick
  (params (DeltaSeconds :type Float%20%28single-precision%29)))

(fn ConstructionScript)

(fn UpdateHealthPoints
  (params (Delta :type Float%20%28double-precision%29))
  ;[0.15 0.15 0.15 0.5] Retire des PDC
  (Variables|Default|SetHealthPoints (+ Delta (Variables|Default|GetHealthPoints)))
  (return 0.0))